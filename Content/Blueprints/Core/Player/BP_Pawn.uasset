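; BP_Pawn is a player camera pawn that moves, rotates in steps and zooms through Enhanced Input actions.
; Forward and right input shift a desired location along the actor's axes, while rotate actions turn a desired rotation in 45-degree increments.
; Tick eases the actor toward both targets with VInterpTo and RInterpTo, without sweep.
; Zoom directly adjusts the spring arm length within a clamped range.
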(event `self.ReceiveBeginPlay`
  (set `self.DesiredLocation` (`self.K2_GetActorLocation`))
  (set `self.DesiredRotation` (`self.K2_GetActorRotation`)))

(event `self.ReceiveTick`
  (params (DeltaSeconds :type "Float (single-precision)"))
  (`self.K2_SetActorLocation` (`KismetMathLibrary.VInterpTo` (`self.K2_GetActorLocation`) (`self.DesiredLocation`) DeltaSeconds 5.0))
  (`self.K2_SetActorRotation` (`KismetMathLibrary.RInterpTo` (`self.K2_GetActorRotation`) (`self.DesiredRotation`) DeltaSeconds 10.0)))

(event `EnhancedInput|/Game/Blueprints/Core/Input/IA_Zoom`
  (params (ActionValue :type "Float (double-precision)") (ElapsedSeconds :type "Float (double-precision)") (TriggeredSeconds :type "Float (double-precision)") (InputAction :type "InputAction Object Reference" :default "/Game/Blueprints/Core/Input/IA_Zoom.IA_Zoom"))
  (bind _springarm (`self.SpringArm`))
  ; Camera Zoom
  (:`Triggered`
    (set `SpringArmComponent.TargetArmLength` (`KismetMathLibrary.FClamp` (- (`SpringArmComponent.TargetArmLength` _springarm) (* ActionValue 20.0)) 100.0 2500.0) _springarm)))

(event `EnhancedInput|/Game/Blueprints/Core/Input/IA_CameraForward`
  (params (ActionValue :type "Float (double-precision)") (ElapsedSeconds :type "Float (double-precision)") (TriggeredSeconds :type "Float (double-precision)") (InputAction :type "InputAction Object Reference" :default "/Game/Blueprints/Core/Input/IA_CameraForward.IA_CameraForward"))
  ; Camera Movement
  (:`Triggered`
    (set `self.DesiredLocation` (+ (`self.DesiredLocation`) (* (* ActionValue 20.0) (`self.GetActorForwardVector`))))))

(event `EnhancedInput|/Game/Blueprints/Core/Input/IA_CameraRight`
  (params (ActionValue :type "Float (double-precision)") (ElapsedSeconds :type "Float (double-precision)") (TriggeredSeconds :type "Float (double-precision)") (InputAction :type "InputAction Object Reference" :default "/Game/Blueprints/Core/Input/IA_CameraRight.IA_CameraRight"))
  ; Camera Movement
  (:`Triggered`
    (set `self.DesiredLocation` (+ (`self.DesiredLocation`) (* (* ActionValue 20.0) (`self.GetActorRightVector`))))))

(event `EnhancedInput|/Game/Blueprints/Core/Input/IA_CameraRotateLeft`
  (params (ActionValue :type Boolean) (ElapsedSeconds :type "Float (double-precision)") (TriggeredSeconds :type "Float (double-precision)") (InputAction :type "InputAction Object Reference" :default "/Game/Blueprints/Core/Input/IA_CameraRotateLeft.IA_CameraRotateLeft"))
  ; Camera Rotate
  (:`Triggered`
    (set `self.DesiredRotation` (`KismetMathLibrary.ComposeRotators` (struct :`Yaw` -45.0) (`self.DesiredRotation`)))))

(event `EnhancedInput|/Game/Blueprints/Core/Input/IA_CameraRotateRight`
  (params (ActionValue :type Boolean) (ElapsedSeconds :type "Float (double-precision)") (TriggeredSeconds :type "Float (double-precision)") (InputAction :type "InputAction Object Reference" :default "/Game/Blueprints/Core/Input/IA_CameraRotateRight.IA_CameraRotateRight"))
  ; Camera Rotate
  (:`Triggered`
    (set `self.DesiredRotation` (`KismetMathLibrary.ComposeRotators` (`self.DesiredRotation`) (struct :`Yaw` 45.0)))))

(fn `UserConstructionScript`)